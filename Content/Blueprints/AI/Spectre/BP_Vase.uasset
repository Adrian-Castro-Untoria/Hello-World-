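; BP_Vase is a vase bound to a linked enemy, apparently a Spectre, that kills that enemy when struck by the trident.
; Each tick it feeds the vase top and enemy locations to a link VFX, with PosMain set to the vase and PosVase to the enemy.
; A TridentV2 capsule overlap calls CallDead, then destroys both enemy and vase only if the enemy is valid.
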(event OnComponentBeginOverlap(Capsule)
  (params (OverlappedComponent :type Primitive%20Component%20Object%20Reference) (OtherActor :type Actor%20Object%20Reference) (OtherComp :type Primitive%20Component%20Object%20Reference) (OtherBodyIndex :type Integer) (bFromSweep :type Boolean) (SweepResult :type Hit%20Result%20Structure%20%28by%20ref%29))
  (bind _linkedenemy (Variables|Default|GetLinkedenemy))
  (Utilities|Casting|CastToTridentV2 OtherActor)
  (Default|CallDead)
  (Utilities|IsValid _linkedenemy
    (:Is%20Valid
      (Actor|DestroyActor _linkedenemy)
      (Actor|DestroyActor))))

(event EventBeginPlay)

(event EventTick
  (params (DeltaSeconds :type Float%20%28single-precision%29))
  (bind _vfx_liaisonincoonu (Variables|Default|GetVFX_Liaisonincoonu))
  (Niagara|SetNiagaraVariable(Vector3) _vfx_liaisonincoonu "PosMain" (Transformation|GetWorldLocation (Variables|Default|GetTopDeVase)))
  (Niagara|SetNiagaraVariable(Vector3) _vfx_liaisonincoonu "PosVase" (Transformation|GetActorLocation (Variables|Default|GetLinkedenemy))))

(fn ConstructionScript)