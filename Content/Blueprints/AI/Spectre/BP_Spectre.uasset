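; BP_Spectre is an AI enemy that endlessly chases the first player character and damages it on contact.
; SpoopyAttaque starts on BeginPlay, runs AI MoveTo toward the player and calls itself again on both success and failure.
; When the Box component begins overlapping a BP_FirstPersonCharacter, it applies damage through a DoOnce gate that resets after a short delay, acting as a hit cooldown.
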(event OnComponentBeginOverlap(Box)
  (params (OverlappedComponent :type Primitive%20Component%20Object%20Reference) (OtherActor :type Actor%20Object%20Reference) (OtherComp :type Primitive%20Component%20Object%20Reference) (OtherBodyIndex :type Integer) (bFromSweep :type Boolean) (SweepResult :type Hit%20Result%20Structure%20%28by%20ref%29))
  (bind _asbp_first_person_character (Utilities|Casting|CastToBP_FirstPersonCharacter OtherActor))
  (Utilities|FlowControl|DoOnce false :!label _label
    (:Completed
      (Game|Damage|ApplyDamage _asbp_first_person_character 1.0 0 0)
      (Utilities|FlowControl|Delay 2.0)
      (goto _label Reset))))

(event Custom|SpoopyAttaque
  (bind _returnvalue (Game|GetPlayerCharacter 0))
  (AI|AIMoveTo self (Transformation|GetActorLocation _returnvalue) _returnvalue 1e+02 false
    (:OnSuccess
      _)
    (:OnFail
      _))
  (CallFunction|SpoopyAttaque))

(event EventBeginPlay
  (CallFunction|SpoopyAttaque))

(fn ConstructionScript)