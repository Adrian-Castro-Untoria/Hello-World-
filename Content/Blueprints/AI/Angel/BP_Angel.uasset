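; BP_Angel is an AI character that chases player 0 and can be frozen in place when seen.
; Despite its name, RandomRoam uses AI MoveTo toward the player and restarts itself on success or failure from BeginPlay onward; the random-point node is unconnected.
; ToggleMouvement takes an IsSeen flag, disabling CharacterMovement when true and restoring walking when false, with no caller in this graph.
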(event Custom|RandomRoam
  (bind _returnvalue (Game|GetPlayerCharacter 0))
  (AI|AIMoveTo self (Transformation|GetActorLocation _returnvalue) _returnvalue 5e+01 false
    (:OnSuccess
      _)
    (:OnFail
      _))
  (CallFunction|RandomRoam))

(event EventBeginPlay
  (CallFunction|RandomRoam))

(event EventToggleMouvement
  (params (IsSeen? :type Boolean))
  (bind _charactermovement (Variables|Character|GetCharacterMovement))
  (if IsSeen?
    (Pawn|Components|CharacterMovement|DisableMovement _charactermovement)
    (else
      (Pawn|Components|CharacterMovement|SetMovementMode _charactermovement "MOVE_Walking" 0))))

(fn ConstructionScript)