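; BP_Diablotin is an AI enemy that takes trident damage and splits into smaller enemies on death.
; Capsule overlaps with TridentV2 subtract its damage from Health and add it to the "Degats" material parameter to show damage.
; At zero Health, it spawns a BP_DiablotinMini running BT_Diablotin at each of three sphere components, then destroys itself.
; JumpAttack uses timelines to lift the StaticMesh component and lower it after a short delay.
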(event OnComponentBeginOverlap(Capsule)
  (params (OverlappedComponent :type Primitive%20Component%20Object%20Reference) (OtherActor :type Actor%20Object%20Reference) (OtherComp :type Primitive%20Component%20Object%20Reference) (OtherBodyIndex :type Integer) (bFromSweep :type Boolean) (SweepResult :type Hit%20Result%20Structure%20%28by%20ref%29))
  (bind _astrident_v2 (Utilities|Casting|CastToTridentV2 OtherActor))
  (bind _output_get (Variables|Default|SetParameter%20Value%20Texture (+ (Variables|/Game/FirstPerson/Blueprints/TridentV2.TridentV2_C|GetDamage _astrident_v2) (Variables|Default|GetParameter%20Value%20Texture))))
  (Rendering|Material|SetScalarParameterValueonMaterials (Variables|Character|GetMesh) "Degats" _output_get)
  (Variables|Default|SetHealth (- (Variables|Default|GetHealth) (Variables|/Game/FirstPerson/Blueprints/TridentV2.TridentV2_C|GetDamage _astrident_v2)))
  (if (<= (Variables|Default|GetHealth) 0.0)
    (for _array_element (Utilities|Array|MakeArray (Variables|Default|GetSphere) (Variables|Default|GetSphere1) (Variables|Default|GetSphere2))
      (AI|SpawnAIFromClass "/Game/Blueprints/AI/Diablotin/BP_DiablotinMini.BP_DiablotinMini_C" "/Game/Blueprints/AI/Diablotin/BT_Diablotin.BT_Diablotin" (.location (Transformation|GetWorldTransform _array_element)) (.rotation (Transformation|GetWorldTransform _array_element)) false 0))
    (Actor|DestroyActor)))

(event Custom|JumpAttack
  (Components|Timeline|SetPlayRate (Variables|Default|GetAttackFinish) 2.0)
  (bind _newtrack_0 (Timeline|AttackFinish PlayFromStart)
    (:Update
      (Transformation|SetRelativeLocation (Variables|Default|GetStaticMesh) (Math|Vector|Lerp(Vector) "-18.000000,0.000000,18.000000" "0.000000,0.000000,350.000000" _newtrack_0) false false))
    (:Finished
      (Utilities|FlowControl|Delay 0.2)
      (Components|Timeline|SetPlayRate (Variables|Default|GetTimeline) 2.0)
      (bind _newtrack_0_2 (Timeline|Timeline ReverseFromEnd)
        (:Update
          (Transformation|SetRelativeLocation (Variables|Default|GetStaticMesh) (Math|Vector|Lerp(Vector) "-18.000000,0.000000,18.000000" "0.000000,0.000000,350.000000" _newtrack_0_2) false false))))))

(event EventBeginPlay
  (Rendering|Material|SetMaterial (Variables|Character|GetMesh) 0 "/Game/Blueprints/AI/Diablotin/M_Diabloin_Inst.M_Diabloin_Inst")
  (Rendering|Material|SetMaterial (Variables|Character|GetMesh) 1 "/Game/Blueprints/AI/Diablotin/M_Diabloin_Inst.M_Diabloin_Inst")
  (Rendering|Material|SetScalarParameterValueonMaterials (Variables|Character|GetMesh) "Degats" (Variables|Default|GetParameter%20Value%20Texture)))

(fn ConstructionScript)