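; Bull AI hazard (Taureau) that charges when the player enters its trigger box and deals damage on contact with its DAMAGE volume.
; A timeline pushes the Cube along the Arrow's forward vector until a DISTANCE delay stops it and flips its rotation between plus and minus 90 degrees.
; The Fini flag blocks retriggering mid-charge, and Tourner tracks the facing.
; A second timeline movement is never run.
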(event OnComponentBeginOverlap(DAMAGE)
  (params (OverlappedComponent :type Primitive%20Component%20Object%20Reference) (OtherActor :type Actor%20Object%20Reference) (OtherComp :type Primitive%20Component%20Object%20Reference) (OtherBodyIndex :type Integer) (bFromSweep :type Boolean) (SweepResult :type Hit%20Result%20Structure%20%28by%20ref%29))
  (bind _asbp_first_person_character (Utilities|Casting|CastToBP_FirstPersonCharacter OtherActor))
  (Game|Damage|ApplyDamage _asbp_first_person_character 1.0 0 0))

(event OnComponentBeginOverlap(Box)
  (params (OverlappedComponent :type Primitive%20Component%20Object%20Reference) (OtherActor :type Actor%20Object%20Reference) (OtherComp :type Primitive%20Component%20Object%20Reference) (OtherBodyIndex :type Integer) (bFromSweep :type Boolean) (SweepResult :type Hit%20Result%20Structure%20%28by%20ref%29))
  (bind _cube (Variables|Default|GetCube))
  (bind _returnvalue (Transformation|GetWorldLocation _cube))
  (if (Variables|Default|Getfini)
    (Variables|Default|Setfini false)
    (Utilities|Casting|CastToBP_FirstPersonCharacter OtherActor)
    (bind _newtrack_0 (Timeline|Movetimeline PlayFromStart)
      (:Update
        (Transformation|SetWorldLocation (Variables|Default|GetCube) (Math|Vector|Lerp(Vector) _returnvalue (+ _returnvalue (* (Math|Vector|GetForwardVector (Variables|Default|GetArrow)) 1.2e+02)) _newtrack_0) false false)
        (Utilities|FlowControl|Delay (Variables|Default|GetDISTANCE))
        (if (Variables|Default|GetTourner)
          (Transformation|SetRelativeRotation (Variables|Default|GetCube) "0.000000,-90.000000,0.000000" false false)
          (Variables|Default|SetTourner false)
          (Variables|Default|Setfini true)
          (Timeline|Movetimeline Stop)
          (else
            (Transformation|SetRelativeRotation (Variables|Default|GetCube) "0.000000,90.000000,0.000000" false false)
            (Variables|Default|SetTourner true)
            (Variables|Default|Setfini true)
            (Timeline|Movetimeline Stop)))))
    (else
      (Utilities|FlowControl|Delay 4.0))))

(fn ConstructionScript)