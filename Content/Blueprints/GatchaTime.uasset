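; Gacha roulette actor that spins once when the player overlaps its box, deducting SoulsPoints from BP_FirstPersonCharacter without checking the balance.
; SpinTheWheel animates the handle with chained timelines and picks one of six prize events by comparing a random roll to cumulative Chance thresholds.
; Each prize timeline spins the wheel with random yaw jitter, snaps it to a fixed angle, then grants souls, health or nothing.
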(event OnComponentBeginOverlap(Box)
  (params (OverlappedComponent :type Primitive%20Component%20Object%20Reference) (OtherActor :type Actor%20Object%20Reference) (OtherComp :type Primitive%20Component%20Object%20Reference) (OtherBodyIndex :type Integer) (bFromSweep :type Boolean) (SweepResult :type Hit%20Result%20Structure%20%28by%20ref%29))
  (bind _as_bp_first_person_character (Variables|Default|GetAs%20BP%20First%20Person%20Character))
  (if (== OtherActor (Game|GetPlayerCharacter 0))
    (Utilities|FlowControl|DoOnce false
      (:Completed
        (CallFunction|SpintheWheel)
        (Variables|/Game/FirstPerson/Blueprints/BP_FirstPersonCharacter.BP_FirstPersonCharacter_C|SetSouls_Points _as_bp_first_person_character (- (Variables|/Game/FirstPerson/Blueprints/BP_FirstPersonCharacter.BP_FirstPersonCharacter_C|GetSouls_Points _as_bp_first_person_character) 15))))))

(event Custom|SpinTheWheel
  (Variables|Default|SetLuckyNumber (Math|Random|RandomIntegerinRange 1 100))
  (CallFunction|Handle)
  (if (<= (Variables|Default|GetLuckyNumber) (Variables|Default|GetChance01))
    (CallFunction|Prize01)
    (elif (<= (Variables|Default|GetLuckyNumber) (+ (Variables|Default|GetChance01) (Variables|Default|GetChance02)))
      (CallFunction|Prize02)
      (elif (<= (Variables|Default|GetLuckyNumber) (+ (Variables|Default|GetChance01) (Variables|Default|GetChance02) (Variables|Default|GetChance03)))
        (CallFunction|Prize03)
        (elif (<= (Variables|Default|GetLuckyNumber) (+ (Variables|Default|GetChance01) (Variables|Default|GetChance02) (Variables|Default|GetChance03) (Variables|Default|GetChance04)))
          (CallFunction|Prize04)
          (elif (<= (Variables|Default|GetLuckyNumber) (+ (Variables|Default|GetChance01) (Variables|Default|GetChance02) (Variables|Default|GetChance03) (Variables|Default|GetChance04) (Variables|Default|GetChance05)))
            (CallFunction|Prize05)
            (else
              (CallFunction|Prize06))))))))

(event Custom|Prize01
  (bind _as_bp_first_person_character (Variables|Default|GetAs%20BP%20First%20Person%20Character))
  (bind _newtrack_0 (Timeline|Timeline_1 PlayFromStart)
    (:Update
      (Transformation|SetRelativeRotation (Variables|Default|GetRoulette) (Math|Rotator|MakeRotator 0.0 0.0 (- _newtrack_0 (Math|Random|RandomFloatinRange 9e+01 1.8e+02))) false false))
    (:Finished
      (Transformation|SetRelativeRotation (Variables|Default|GetRoulette) (Math|Rotator|MakeRotator 0.0 0.0 75.0) false false)
      (Variables|/Game/FirstPerson/Blueprints/BP_FirstPersonCharacter.BP_FirstPersonCharacter_C|SetSouls_Points _as_bp_first_person_character (+ (Variables|/Game/FirstPerson/Blueprints/BP_FirstPersonCharacter.BP_FirstPersonCharacter_C|GetSouls_Points _as_bp_first_person_character) 30)))))

(event Custom|Prize02
  (bind _newtrack_0 (Timeline|Timeline_2 PlayFromStart)
    (:Update
      (Transformation|SetRelativeRotation (Variables|Default|GetRoulette) (Math|Rotator|MakeRotator 0.0 0.0 (- _newtrack_0 (Math|Random|RandomFloatinRange 9e+01 1.8e+02))) false false))
    (:Finished
      (Transformation|SetRelativeRotation (Variables|Default|GetRoulette) (Math|Rotator|MakeRotator 0.0 0.0 -1.5e+02) false false)
      (Variables|/Game/FirstPerson/Blueprints/BP_FirstPersonCharacter.BP_FirstPersonCharacter_C|SetHealth (Variables|Default|GetAs%20BP%20First%20Person%20Character) 4.0))))

(event Custom|Prize03
  (bind _as_bp_first_person_character (Variables|Default|GetAs%20BP%20First%20Person%20Character))
  (bind _newtrack_0 (Timeline|Timeline_3 PlayFromStart)
    (:Update
      (Transformation|SetRelativeRotation (Variables|Default|GetRoulette) (Math|Rotator|MakeRotator 0.0 0.0 (- _newtrack_0 (Math|Random|RandomFloatinRange 9e+01 1.8e+02))) false false))
    (:Finished
      (Transformation|SetRelativeRotation (Variables|Default|GetRoulette) (Math|Rotator|MakeRotator 0.0 0.0 -15.0) false false)
      (Variables|/Game/FirstPerson/Blueprints/BP_FirstPersonCharacter.BP_FirstPersonCharacter_C|SetHealth _as_bp_first_person_character (+ (Variables|/Game/FirstPerson/Blueprints/BP_FirstPersonCharacter.BP_FirstPersonCharacter_C|GetHealth _as_bp_first_person_character) 2.0))
      (if (> (Variables|/Game/FirstPerson/Blueprints/BP_FirstPersonCharacter.BP_FirstPersonCharacter_C|GetHealth _as_bp_first_person_character) 4.0)
        (Variables|/Game/FirstPerson/Blueprints/BP_FirstPersonCharacter.BP_FirstPersonCharacter_C|SetHealth _as_bp_first_person_character 4.0)))))

(event Custom|Prize04
  (bind _as_bp_first_person_character (Variables|Default|GetAs%20BP%20First%20Person%20Character))
  (bind _newtrack_0 (Timeline|Timeline_4 PlayFromStart)
    (:Update
      (Transformation|SetRelativeRotation (Variables|Default|GetRoulette) (Math|Rotator|MakeRotator 0.0 0.0 (- _newtrack_0 (Math|Random|RandomFloatinRange 9e+01 1.8e+02))) false false))
    (:Finished
      (Transformation|SetRelativeRotation (Variables|Default|GetRoulette) (Math|Rotator|MakeRotator 0.0 0.0 35.0) false false)
      (Variables|/Game/FirstPerson/Blueprints/BP_FirstPersonCharacter.BP_FirstPersonCharacter_C|SetHealth _as_bp_first_person_character (+ (Variables|/Game/FirstPerson/Blueprints/BP_FirstPersonCharacter.BP_FirstPersonCharacter_C|GetHealth _as_bp_first_person_character) 1.0))
      (if (> (Variables|/Game/FirstPerson/Blueprints/BP_FirstPersonCharacter.BP_FirstPersonCharacter_C|GetHealth _as_bp_first_person_character) 4.0)
        (Variables|/Game/FirstPerson/Blueprints/BP_FirstPersonCharacter.BP_FirstPersonCharacter_C|SetHealth _as_bp_first_person_character 4.0)))))

(event Custom|Prize05
  (bind _as_bp_first_person_character (Variables|Default|GetAs%20BP%20First%20Person%20Character))
  (bind _newtrack_0 (Timeline|Timeline_5 PlayFromStart)
    (:Update
      (Transformation|SetRelativeRotation (Variables|Default|GetRoulette) (Math|Rotator|MakeRotator 0.0 0.0 (- _newtrack_0 (Math|Random|RandomFloatinRange 9e+01 1.8e+02))) false false))
    (:Finished
      (Transformation|SetRelativeRotation (Variables|Default|GetRoulette) (Math|Rotator|MakeRotator 0.0 0.0 -105.0) false false)
      (Variables|/Game/FirstPerson/Blueprints/BP_FirstPersonCharacter.BP_FirstPersonCharacter_C|SetSouls_Points _as_bp_first_person_character (+ (Variables|/Game/FirstPerson/Blueprints/BP_FirstPersonCharacter.BP_FirstPersonCharacter_C|GetSouls_Points _as_bp_first_person_character) 5)))))

(event Custom|Prize06
  (bind _newtrack_0 (Timeline|Timeline_6 PlayFromStart)
    (:Update
      (Transformation|SetRelativeRotation (Variables|Default|GetRoulette) (Math|Rotator|MakeRotator 0.0 0.0 (- _newtrack_0 (Math|Random|RandomFloatinRange 9e+01 1.8e+02))) false false))
    (:Finished
      (Transformation|SetRelativeRotation (Variables|Default|GetRoulette) (Math|Rotator|MakeRotator 0.0 0.0 1.5e+02) false false))))

(event Custom|Handle
  (bind _manchesphere (Variables|Default|GetMancheSphere))
  (Components|Timeline|SetPlayRate (Variables|Default|GetTimeline) 1.0)
  (bind _newtrack_0 (Timeline|Timeline PlayFromStart)
    (:Update
      (Transformation|SetRelativeRotation _manchesphere (Math|Rotator|Lerp(Rotator) (Variables|/Script/Engine.SceneComponent|GetRelativeRotation _manchesphere) "0.000000,0.000000,-75.000000" _newtrack_0) false false))
    (:Finished
      (Components|Timeline|SetPlayRate (Variables|Default|GetTimeline_0) 2.0)
      (bind _newtrack_0_2 (Timeline|Timeline_0 PlayFromStart)
        (:Update
          (Transformation|SetRelativeRotation (Variables|Default|GetMancheSphere) (Math|Rotator|Lerp(Rotator) "0.000000,0.000000,-75.000000" "0, 0, 0" _newtrack_0_2) false false))))))

(event EventBeginPlay
  (bind _asbp_first_person_character (Utilities|Casting|CastToBP_FirstPersonCharacter (Game|GetPlayerCharacter 0)))
  (Variables|Default|SetAs%20BP%20First%20Person%20Character _asbp_first_person_character)
  (Variables|Default|SetRelative%20Rotation (Variables|/Script/Engine.SceneComponent|GetRelativeRotation (Variables|Default|GetRoulette))))

(event Collision|EventActorBeginOverlap
  (params (OtherActor :type Actor%20Object%20Reference)))

(event EventTick
  (params (DeltaSeconds :type Float%20%28single-precision%29)))

(fn ConstructionScript)